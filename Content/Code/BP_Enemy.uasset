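; Patrolling enemy with a Clean or Dirty state, shown by its material, that only harms or can be stomped by a player in a differing state.
; If mobile, it moves between two detached target components, reversing direction on the Y axis.
; Weapon overlap destroys a differing player, while Tick rechecks a matching one in case their states diverge.
; WeakSpot overlap bounces a differing player, then flattens, disarms and destroys the enemy after a delay.
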(event `self.ReceiveBeginPlay`
  (`SceneComponent.K2_DetachFromComponent` (`self.Target_Left`) "KeepWorld" "KeepWorld" "KeepWorld" true)
  (`SceneComponent.K2_DetachFromComponent` (`self.Target_Right`) "KeepWorld" "KeepWorld" "KeepWorld" true)
  (switch `/Game/Code/BP_DisgustState` (`self.DisgustState`)
    (:`NewEnumerator0`
      (`PrimitiveComponent.SetMaterial` (`self.StaticMesh`) 0 "/Game/Materials/MI_Clean.MI_Clean"))
    (:`NewEnumerator1`
      (`PrimitiveComponent.SetMaterial` (`self.StaticMesh`) 0 "/Game/Materials/MI_Dirty.MI_Dirty"))))

(event `self.ReceiveTick`
  (params (DeltaSeconds :type "Float (single-precision)"))
  (`self.UpdateLocation` DeltaSeconds)
  (`self.CheckDestroyOverlapping`)
  (bind _returnvalue (`self.IsInvertNecessary`))
  (if _returnvalue
    (`self.InvertMovement`)))

(event `self.Weapon.OnComponentEndOverlap`
  (params (OverlappedComponent :type "PrimitiveComponent Object Reference") (OtherActor :type "Actor Object Reference") (OtherComp :type "PrimitiveComponent Object Reference") (OtherBodyIndex :type Integer))
  (set `self.IsOverlapping` false))

(event `self.Weapon.OnComponentBeginOverlap`
  (params (OverlappedComponent :type "PrimitiveComponent Object Reference") (OtherActor :type "Actor Object Reference") (OtherComp :type "PrimitiveComponent Object Reference") (OtherBodyIndex :type Integer) (bFromSweep :type Boolean) (SweepResult :type "HitResult Structure (by ref)"))
  (bind _asbp_player (cast `/Game/Code/BP_Player` OtherActor))
  (if (`self.IsNotDisgusting` _asbp_player)
    (set `self.OverlappingWith` _asbp_player)
    (set `self.IsOverlapping` true)
    (else
      (`self.K2_DestroyActor` _asbp_player))))

(event `self.WeakSpot.OnComponentBeginOverlap`
  (params (OverlappedComponent :type "PrimitiveComponent Object Reference") (OtherActor :type "Actor Object Reference") (OtherComp :type "PrimitiveComponent Object Reference") (OtherBodyIndex :type Integer) (bFromSweep :type Boolean) (SweepResult :type "HitResult Structure (by ref)"))
  (bind _asbp_player (cast `/Game/Code/BP_Player` OtherActor))
  (if (not (`self.IsNotDisgusting` _asbp_player))
    (`/Game/Code/BP_Player.Bounce` _asbp_player)
    (`self.SetActorScale3D` (1.0 1.0 0.3))
    (set `self.MoveSpeed` 0.0)
    (`ActorComponent.K2_DestroyComponent` (`self.Weapon`))
    (`PrimitiveComponent.SetCollisionEnabled` (`self.WeakSpot`) "NoCollision")
    (`KismetSystemLibrary.Delay` 1.0)
    (`self.K2_DestroyActor`)))

(fn `CheckDestroyOverlapping`
  (bind _overlappingwith (`self.OverlappingWith`))
  (if (`self.IsOverlapping`)
    (if (not (`self.IsNotDisgusting` _overlappingwith))
      (`self.K2_DestroyActor` _overlappingwith))))

(fn `InvertMovement`
  (set `self.MoveDirection` (* (`self.MoveDirection`) -1.0)))

(fn `IsInvertNecessary`
  (returns (ReturnValue :type Boolean))
  (return (or (and (`self.IsMovingRight`) (`self.IsPastRightTarget`)) (and (`self.IsMovingLeft`) (`self.IsPastLeftTarget`)))))

(fn `IsMovingLeft`
  (returns (ReturnValue :type Boolean))
  (bind (_movedirection_x _movedirection_y) (`KismetMathLibrary.BreakVector` (`self.MoveDirection`)))
  (return (< _movedirection_y 0.0)))

(fn `IsMovingRight`
  (returns (ReturnValue :type Boolean))
  (bind (_movedirection_x _movedirection_y) (`KismetMathLibrary.BreakVector` (`self.MoveDirection`)))
  (return (> _movedirection_y 0.0)))

(fn `IsNotDisgusting`
  (params (Player :type "/Game/Code/BP_Player Object Reference"))
  (returns (IsNotDisgusting :type Boolean))
  (return (`|EnumEquality` (`/Game/Code/BP_Player.DisgustState` Player) (`self.DisgustState`))))

(fn `IsPastLeftTarget`
  (returns (ReturnValue :type Boolean))
  (bind (_returnvalue_x _returnvalue_y) (`KismetMathLibrary.BreakVector` (`self.K2_GetActorLocation`)))
  (bind (_returnvalue_x_2 _returnvalue_y_2) (`KismetMathLibrary.BreakVector` (`SceneComponent.K2_GetComponentLocation` (`self.Target_Left`))))
  (return (< _returnvalue_y _returnvalue_y_2)))

(fn `IsPastRightTarget`
  (returns (ReturnValue :type Boolean))
  (bind (_returnvalue_x _returnvalue_y) (`KismetMathLibrary.BreakVector` (`self.K2_GetActorLocation`)))
  (bind (_returnvalue_x_2 _returnvalue_y_2) (`KismetMathLibrary.BreakVector` (`SceneComponent.K2_GetComponentLocation` (`self.Target_Right`))))
  (return (> _returnvalue_y _returnvalue_y_2)))

(fn `UpdateLocation`
  (params (DeltaSeconds :type "Float (double-precision)"))
  (if (`self.IsMobile`)
    (`self.K2_SetActorLocation` (+ (`self.K2_GetActorLocation`) (* (`self.MoveDirection`) (* DeltaSeconds (`self.MoveSpeed`)))))))

(fn `UserConstructionScript`)