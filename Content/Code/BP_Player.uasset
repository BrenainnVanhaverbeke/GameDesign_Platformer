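; BP_Player is a physics-capsule player character that moves along the Y axis, jumps, bounces and can get a temporary speed boost.
; Jump applies an impulse when a downward sphere trace hits, while movement offsets the actor's location by WalkSpeed without sweeping.
; MoveLeft and MoveRight presses switch DisgustState and the clean or dirty mesh material.
; Tick times out the boost, and destruction reloads the current level.
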(event `InputAction|Jump`
  (params (Key :type "Key Structure"))
  (:`Pressed`
    (`self.Jump`)))

(event `InputAxis|MoveCharacter`
  (params (AxisValue :type "Float (single-precision)"))
  (`self.MoveCharacter` AxisValue))

(event `InputAction|MoveLeft`
  (params (Key :type "Key Structure"))
  (:`Pressed`
    (set `self.DisgustState` "NewEnumerator0")
    (`PrimitiveComponent.SetMaterial` (`self.StaticMesh`) 0 "/Game/Materials/MI_Clean.MI_Clean")))

(event `InputAction|MoveRight`
  (params (Key :type "Key Structure"))
  (:`Pressed`
    (set `self.DisgustState` "NewEnumerator1")
    (`PrimitiveComponent.SetMaterial` (`self.StaticMesh`) 0 "/Game/Materials/MI_Dirty.MI_Dirty")))

(event `self.ReceiveDestroyed`
  (bind _returnvalue (`GameplayStatics.GetCurrentLevelName` true))
  (`GameplayStatics.OpenLevel` (`KismetStringLibrary.Conv_StringToName` _returnvalue)))

(event `self.ReceiveBeginPlay`
  (set `self.WalkSpeed` (`self.DefaultWalkSpeed`)))

(event `self.ReceiveTick`
  (params (DeltaSeconds :type "Float (single-precision)"))
  (`self.HandleFastTime` DeltaSeconds))

(fn `Bounce`
  (`PrimitiveComponent.SetPhysicsLinearVelocity` (`self.Capsule`) (`KismetMathLibrary.MakeVector` 0.0 0.0 (/ (`self.JumpStrength`) 2.0)) false "None"))

(fn `HandleFastTime`
  (params (DeltaSeconds :type "Float (double-precision)"))
  (if (`self.IsSpedUp`)
    (set `self.FastTime` (+ DeltaSeconds (`self.FastTime`)))
    (if (`self.IsFastTimeExpired`)
      (set `self.WalkSpeed` (`self.DefaultWalkSpeed`))
      (set `self.IsSpedUp` false)
      (`KismetSystemLibrary.PrintString` "OH SHIIIIIT! I'M SLOWING DOWN!"))))

(fn `IsFastTimeExpired`
  (returns (ReturnValue :type Boolean))
  (return (< (`self.MaxFastTime`) (`self.FastTime`))))

(fn `Jump`
  (bind _returnvalue (`self.K2_GetActorLocation`))
  (bind _capsule (`self.Capsule`))
  (bind (_outhit _returnvalue_2) (`KismetSystemLibrary.SphereTraceSingle` :`Start` _returnvalue :`End` (- _returnvalue (`KismetMathLibrary.MakeVector` 0.0 0.0 (`CapsuleComponent.CapsuleHalfHeight` _capsule))) :`Radius` (`CapsuleComponent.CapsuleRadius` _capsule) :`TraceChannel` "TraceTypeQuery1" :`DrawDebugType` "ForDuration"))
  (if _returnvalue_2
    (`PrimitiveComponent.AddImpulse` (`self.Capsule`) (`KismetMathLibrary.MakeVector` 0.0 0.0 (`self.JumpStrength`)) "None" true)))

(fn `MoveCharacter`
  (params (AxisValue :type "Float (double-precision)"))
  (`self.K2_SetActorLocation` (+ (* (* (`KismetMathLibrary.MakeVector` 0.0 (`self.WalkSpeed`)) AxisValue) (`GameplayStatics.GetWorldDeltaSeconds`)) (`self.K2_GetActorLocation`))))

(fn `SpeedUp`
  (set `self.WalkSpeed` (`self.FastWalkSpeed`))
  (set `self.FastTime` 0.0)
  (set `self.IsSpedUp` true)
  (`KismetSystemLibrary.PrintString` "SPEEDWEED! YAY!"))

(fn `UserConstructionScript`)