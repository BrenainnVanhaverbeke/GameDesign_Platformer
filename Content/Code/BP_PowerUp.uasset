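; BP_PowerUp is a moving pickup that calls SpeedUp on the player that overlaps it, then destroys itself.
; It spawns moving along a spawn direction until it rises above OnSpawnTarget, a component detached at BeginPlay to hold its world position.
; It then switches to its normal direction and speed and enables sphere physics constrained to the YZ plane, while Tick keeps applying the manual movement.
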(event `self.ReceiveBeginPlay`
  (set `self.MoveDirection` (`self.SpawnDirection`))
  (set `self.MoveSpeed` (`self.SpawnSpeed`))
  (`SceneComponent.K2_DetachFromComponent` (`self.OnSpawnTarget`) "KeepWorld" "KeepWorld" "KeepRelative" true))

(event `self.ReceiveTick`
  (params (DeltaSeconds :type "Float (single-precision)"))
  (`self.MovePowerUp` DeltaSeconds)
  (if (not (`self.IsDoneSpawning`))
    (`self.CheckDoneSpawning`)
    (if (`self.IsDoneSpawning`)
      (`self.InitialiseNormalMove`))))

(event `self.ReceiveActorBeginOverlap`
  (params (OtherActor :type "Actor Object Reference"))
  (bind _asbp_player (cast `/Game/Code/BP_Player` OtherActor))
  (`/Game/Code/BP_Player.SpeedUp` _asbp_player)
  (`self.K2_DestroyActor`))

(fn `CheckDoneSpawning`
  (bind (_returnvalue_x _returnvalue_y _returnvalue_z) (`KismetMathLibrary.BreakVector` (`self.K2_GetActorLocation`)))
  (bind (_returnvalue_x_2 _returnvalue_y_2 _returnvalue_z_2) (`KismetMathLibrary.BreakVector` (`SceneComponent.K2_GetComponentLocation` (`self.OnSpawnTarget`))))
  (set `self.IsDoneSpawning` (> _returnvalue_z _returnvalue_z_2)))

(fn `InitialiseNormalMove`
  (set `self.MoveDirection` (`self.InitialMoveDirection`))
  (set `self.MoveSpeed` (`self.InitialMoveSpeed`))
  (`PrimitiveComponent.SetSimulatePhysics` (`self.Sphere`) true)
  (`PrimitiveComponent.SetConstraintMode` (`self.Sphere`) "YZPlane"))

(fn `MovePowerUp`
  (params (A :type "Float (double-precision)"))
  (`self.K2_SetActorLocation` (+ (`self.K2_GetActorLocation`) (* (`self.MoveDirection`) (* A (`self.MoveSpeed`))))))

(fn `UserConstructionScript`)